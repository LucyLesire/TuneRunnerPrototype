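; BP_SoundMaster runs a rhythm level, playing the selected song and spawning its beats across three music lanes.
; It reads precomputed NRT onsets, drops weak ones and picks each beat's lane by onset-strength tercile, adding periodic obstacles and power-ups in other lanes.
; Spawning leads delayed audio by the lane travel time.
; It also handles tutorial spawns, pitch-matched slow motion and saving stats before the EndGame level.
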(event `self.ReceiveBeginPlay`
  (bind _music (`self.Music`))
  (bind _duration (`SoundBase.Duration` _music))
  (bind (_outonsettimestamps _outonsetstrengths) (`OnsetNRT.GetNormalizedChannelOnsetsBetweenTimes` (`self.OnsetNRT`) 0.0 _duration 0))
  ;[1 1 1] Add different songs
  (`KismetArrayLibrary.Array_Add` (`self.NRTs`) "/Game/Blueprints/Sounds/Sound_OnsetNRT.Sound_OnsetNRT")
  (`KismetArrayLibrary.Array_Add` (`self.NRTs`) "/Game/Blueprints/Sounds/Sound_OnsetNRT_2.Sound_OnsetNRT_2")
  (`KismetArrayLibrary.Array_Add` (`self.NRTs`) "/Game/Blueprints/Sounds/Sound_OnsetNRT_3.Sound_OnsetNRT_3")
  (`KismetArrayLibrary.Array_Add` (`self.NRTs`) "/Game/Blueprints/Sounds/Sound_OnsetNRT_4.Sound_OnsetNRT_4")
  (`KismetArrayLibrary.Array_Add` (`self.NRTs`) "/Game/Blueprints/Sounds/Sound_OnsetNRT_5.Sound_OnsetNRT_5")
  (`KismetArrayLibrary.Array_Add` (`self.NRTs`) "/Game/Blueprints/Sounds/Sound_OnsetNRT_6.Sound_OnsetNRT_6")
  (`KismetArrayLibrary.Array_Add` (`self.NRTs`) "/Game/Blueprints/Sounds/Sound_OnsetNRT_7.Sound_OnsetNRT_7")
  (bind _asbp_game_instance (cast `/Game/Blueprints/Base/BP_GameInstance` (`GameplayStatics.GetGameInstance`)))
  (set `self.Tutorial` (`|EnumEquality` (`/Game/Blueprints/Base/BP_GameInstance.Difficulty` _asbp_game_instance) "NewEnumerator3"))
  (set `self.OnsetNRT` (`|GetArrayItem` (`self.NRTs`) (`/Game/Blueprints/Base/BP_GameInstance.CurrentSound` _asbp_game_instance)))
  (bind _outactors (`GameplayStatics.GetAllActorsOfClass` "/Game/Blueprints/Beats/BP_MusicLane.BP_MusicLane_C"))
  (bind _musiclanesout (`self.SortMusicLanes` _outactors))
  (bind _output_get (set `self.MusicLanes` _musiclanesout))
  (bind _output (`|GetArrayItem` _output_get))
  (bind _returnvalue_x (`KismetMathLibrary.BreakVector` (`SceneComponent.K2_GetComponentLocation` (`/Game/Blueprints/Beats/BP_MusicLane.PlayerSocket` _output))))
  (bind _returnvalue_x_2 (`KismetMathLibrary.BreakVector` (`SceneComponent.K2_GetComponentLocation` (`/Game/Blueprints/Beats/BP_MusicLane.BeatSocket` _output))))
  ;[1 1 1] Get distance for beats to travel
  (set `self.DistanceBetweenSockets` (+ (`KismetMathLibrary.Abs` _returnvalue_x) (`KismetMathLibrary.Abs` _returnvalue_x_2)))
  (set `self.Music` (`AudioAnalyzerNRT.Sound` (`self.OnsetNRT`)))
  (`AudioComponent.SetSound` (`self.Audio`) _music)
  (set `self.MusicDuration` _duration)
  (add `AudioComponent.OnAudioPlaybackPercent` (`self.Audio`) (delegate `PlaybackChange`))
  ;[1 1 1] Get beats from audio
  (set `self.OnsetTimeStamps` _outonsettimestamps)
  (`|ExecutionSequence`
    (:`then_0`
      ;[1 1 1] Mark weak onsets for delete
      (bind _output_get_2 (set `self.Out Onset Strengths` _outonsetstrengths))
      (for (_array_element _array_index) _output_get_2
        (if (not (>= _array_element (* (`.MinValue` (`KismetMathLibrary.MinOfFloatArray` _outonsetstrengths)) 4.0)))
          (`KismetArrayLibrary.Array_Add` (`self.MarkForDelete`) _array_index))))
    (:`then_1`
      ;[1 1 1] Remove weak onsets
      (bind (_arrayindex _arrayelement) (`/Engine/EditorBlueprintResources/StandardMacros.ReverseForEachLoop` (`self.MarkForDelete`))
        (:`LoopBody`
          (`KismetArrayLibrary.Array_Remove` (`self.OnsetTimeStamps`) _arrayelement)
          (`KismetArrayLibrary.Array_Remove` (`self.Out Onset Strengths`) _arrayelement))
        (:`Completed`
          ;[1 1 1] Sort array low to high
          (bind _sortedarray (`self.SortArray` (`self.Out Onset Strengths`)))
          (set `self.SortedArray` _sortedarray)
          (bind _output_get_3 (set `self.WaitTimeBeforePlay` (/ (`self.DistanceBetweenSockets`) 900.0)))
          (set `self.IsWaiting` true)
          (`KismetSystemLibrary.Delay` _output_get_3)
          (`AudioComponent.Play` (`self.Audio`) 0.0))))))

(event `PlaybackChange`
  (params (PlayingSoundWave :type "SoundWave Object Reference") (PlaybackPercent :type "Float (double-precision)"))
  ;[1 1 1] Set played time accordingly
  (set `self.PlayedTime` (* PlaybackPercent (`self.MusicDuration`))))

(event `self.ReceiveTick`
  (params (DeltaSeconds :type "Float (single-precision)"))
  (bind _output (`|GetArrayItem` (`self.OnsetTimeStamps`) (`self.LastBeatHit`)))
  (set `self.TimeSinceLastBeat` (+ DeltaSeconds (`self.TimeSinceLastBeat`)))
  (if (`self.IsWaiting`)
    ;[1 1 1] Make sure the beats hit the player when they occur in song
    (bind _output_get (set `self.PlayedTime` (+ DeltaSeconds (`self.PlayedTime`))))
    (if (>= _output_get (`self.WaitTimeBeforePlay`))
      (set `self.IsWaiting` false)
      (else
        ;[1 1 1] Check if song is over
        (if (>= (+ (`self.LastBeatHit`) 1) (`KismetArrayLibrary.Array_Length` (`self.OnsetTimeStamps`))) :!label _label
          ;[1 1 1] End song
          (`/Engine/EditorBlueprintResources/StandardMacros.DoOnce` false
            (:`Completed`
              (`self.EndOfSong`)))
          (else
            ;[1 1 1] Spawn beat when beat occurs in audio
            (if (`KismetMathLibrary.NearlyEqual_FloatFloat` _output (`self.PlayedTime`) 0.01)
              (if (>= (`self.TimeSinceLastBeat`) (`self.MinTimeBetweenBeats`))
                (`self.SpawnBeat`)
                (set `self.TimeSinceLastBeat` 0.0))
              (`/Engine/EditorBlueprintResources/StandardMacros.IncrementInt` (`self.LastBeatHit`) :!label _label_2
                (:`  `
                  ;[1 1 1] Tutorial sequence
                  (if (`self.Tutorial`)
                    (bind _asbp_game_instance (cast `/Game/Blueprints/Base/BP_GameInstance` (`GameplayStatics.GetGameInstance`)))
                    (bind _currenttutorial (`/Game/Blueprints/Base/BP_GameInstance.CurrentTutorial` _asbp_game_instance))
                    (if (== _currenttutorial 2)
                      (`/Engine/EditorBlueprintResources/StandardMacros.DoOnce` false
                        (:`Completed`
                          (`/Game/Blueprints/Beats/BP_MusicLane.SpawnObstacle` (`|GetArrayItem` (`self.MusicLanes`) (`KismetMathLibrary.RandomIntegerInRange` 1 2)))
                          (`KismetSystemLibrary.Delay` 3.0 :!label _label_3)
                          (`/Engine/EditorBlueprintResources/StandardMacros.IncrementInt` _currenttutorial)))
                      (elif (== _currenttutorial 3)
                        (`/Engine/EditorBlueprintResources/StandardMacros.DoOnce` false
                          (:`Completed`
                            (`/Game/Blueprints/Beats/BP_MusicLane.SpawnPowerUp` (`|GetArrayItem` (`self.MusicLanes`) (`KismetMathLibrary.RandomIntegerInRange` 1 2)))
                            (goto _label_3))))))))
              (elif (>= (`self.PlayedTime`) _output)
                (goto _label_2)))))))
    (else
      (set `self.PlayedTime` (+ (`self.PlayedTime`) (`self.WaitTimeBeforePlay`)))
      (goto _label))))

(event `SpawnBeat`
  (bind _sortedarray (`self.SortedArray`))
  (bind _returnvalue (`KismetArrayLibrary.Array_Length` _sortedarray))
  (bind _output (`|GetArrayItem` (`self.Out Onset Strengths`) (`self.LastBeatHit`)))
  ;[1 1 1] Calculate lane for beat & spawn on correct lane
  (if (<= _output (`|GetArrayItem` _sortedarray (/ _returnvalue 3)))
    ;;[1 1 1] Spawn beat on lane 0
    (`/Game/Blueprints/Beats/BP_MusicLane.SpawnBeats` (`|GetArrayItem` (`self.MusicLanes`)))
    ;[1 1 1] Every 7 beats spawn an obstacle
    (if (== (mod (`self.LastBeatHit`) 7) 5)
      (`self.SpawnObstacle` 0))
    ;[1 1 1] Spawn powerup every 45 beats
    (if (== (mod (`self.LastBeatHit`) 45) 7)
      (`self.SpawnPowerUp` 0))
    (else
      ;;[1 1 1] Spawn beat on lane 1
      (if (<= _output (`|GetArrayItem` _sortedarray (`KismetMathLibrary.Round` (/ (`KismetMathLibrary.Conv_IntToDouble` _returnvalue) 1.5))))
        (`/Game/Blueprints/Beats/BP_MusicLane.SpawnBeats` (`|GetArrayItem` (`self.MusicLanes`) 1))
        ;[1 1 1] Every 7 beats spawn an obstacle
        (if (== (mod (`self.LastBeatHit`) 7) 5)
          (`self.SpawnObstacle` 1))
        ;[1 1 1] Spawn powerup every 45 beats
        (if (== (mod (`self.LastBeatHit`) 45) 7)
          (`self.SpawnPowerUp` 1))
        (else
          ;;[1 1 1] Spawn beat on lane 2
          (`/Game/Blueprints/Beats/BP_MusicLane.SpawnBeats` (`|GetArrayItem` (`self.MusicLanes`) 2))
          ;[1 1 1] Every 7 beats spawn an obstacle
          (if (== (mod (`self.LastBeatHit`) 7) 5)
            (`self.SpawnObstacle` 2))
          ;[1 1 1] Spawn powerup every 45 beats
          (if (== (mod (`self.LastBeatHit`) 45) 7)
            (`self.SpawnPowerUp` 2)))))))

(event `SpawnObstacle`
  (params (CurrentLane :type Integer))
  (bind _musiclanes (`self.MusicLanes`))
  ;[1 1 1] Spawn an obstacle
  (if (`self.Tutorial`)
    _
    (elif (== CurrentLane 0)
      ;;[1 1 1] Spawn on other lane then lane 0
      (`/Game/Blueprints/Beats/BP_MusicLane.SpawnObstacle` (`|GetArrayItem` (`self.MusicLanes`) (`KismetMathLibrary.RandomIntegerInRange` 1 2)))
      (elif (== CurrentLane 1)
        ;;[1 1 1] Spawn on other lane then lane 1
        (if (`KismetMathLibrary.RandomBool`)
          (`/Game/Blueprints/Beats/BP_MusicLane.SpawnObstacle` (`|GetArrayItem` _musiclanes))
          (else
            (`/Game/Blueprints/Beats/BP_MusicLane.SpawnObstacle` (`|GetArrayItem` _musiclanes 2))))
        (else
          ;;[1 1 1] Spawn on other lane then lane 2
          (`/Game/Blueprints/Beats/BP_MusicLane.SpawnObstacle` (`|GetArrayItem` (`self.MusicLanes`) (`KismetMathLibrary.RandomIntegerInRange` 0 1))))))))

(event `EndOfSong`
  ;[1 1 1] End of song => Set stats
  (bind _asbp_player_character_2 (cast `/Game/Blueprints/Player/BP_PlayerCharacter2` (`GameplayStatics.GetPlayerCharacter` 0)))
  (bind _asbp_game_instance (cast `/Game/Blueprints/Base/BP_GameInstance` (`GameplayStatics.GetGameInstance`)))
  (set `/Game/Blueprints/Base/BP_GameInstance.BeatsHit` (`/Game/Blueprints/Player/BP_PlayerCharacter2.BeatsHit` _asbp_player_character_2) _asbp_game_instance)
  (set `/Game/Blueprints/Base/BP_GameInstance.GameOver` false _asbp_game_instance)
  (bind _asbp_game_mode (cast `/Game/Blueprints/Player/BP_GameMode` (`GameplayStatics.GetGameMode`)))
  (set `/Game/Blueprints/Base/BP_GameInstance.FinalScore` (`KismetMathLibrary.FTrunc` (`/Game/Blueprints/Player/BP_GameMode.TimeLeft` _asbp_game_mode)) _asbp_game_instance)
  (`KismetSystemLibrary.Delay` 5.0)
  (`GameplayStatics.OpenLevel` "EndGame"))

(event `SlowDownTime`
  (`/Engine/EditorBlueprintResources/StandardMacros.DoOnce` false :!label _label_4
    (:`Completed`
      (`GameplayStatics.SetGlobalTimeDilation` 0.75)
      (`AudioComponent.SetPitchMultiplier` (`self.Audio`) (`GameplayStatics.GetGlobalTimeDilation`))
      (`KismetSystemLibrary.Delay` 3.75)
      (`GameplayStatics.SetGlobalTimeDilation` 1.0)
      (`AudioComponent.SetPitchMultiplier` (`self.Audio`) (`GameplayStatics.GetGlobalTimeDilation`))
      (goto _label_4 :!via `Reset`))))

(event `SpawnPowerUp`
  (params (CurrentLane :type Integer))
  ;[1 1 1] Spawn powerups
  (if (`self.Tutorial`)
    _
    (elif (== CurrentLane 0)
      ;;[1 1 1] Spawn a powerup on another lane then lane 0
      (`/Game/Blueprints/Beats/BP_MusicLane.SpawnPowerUp` (`|GetArrayItem` (`self.MusicLanes`) (`KismetMathLibrary.RandomIntegerInRange` 1 2)))
      (elif (== CurrentLane 1)
        ;;[1 1 1] Spawn powerup on other lane then lane 1
        (if (`KismetMathLibrary.RandomBool`)
          (`/Game/Blueprints/Beats/BP_MusicLane.SpawnPowerUp` (`|GetArrayItem` (`self.MusicLanes`)))
          (else
            (`/Game/Blueprints/Beats/BP_MusicLane.SpawnPowerUp` (`|GetArrayItem` (`self.MusicLanes`) 2))))
        (else
          ;;[1 1 1] Spawn powerup on other lane then lane 2
          (`/Game/Blueprints/Beats/BP_MusicLane.SpawnPowerUp` (`|GetArrayItem` (`self.MusicLanes`) (`KismetMathLibrary.RandomIntegerInRange` 0 1))))))))

(fn `SortArray`
  (params (inputArray :type "Array of Float (double-precision)"))
  (returns (sortedArray :type "Array of Float (double-precision)"))
  (locals (toBeSorted :type "Array of Float (double-precision)") (sorted :type "Array of Float (double-precision)"))
  (bind _output_get (set `local.toBeSorted` inputArray))
  (while (!= (`KismetArrayLibrary.Array_Length` _output_get) 0)
    (bind (_indexofminvalue _minvalue) (`KismetMathLibrary.MinOfFloatArray` _output_get))
    (`KismetArrayLibrary.Array_Add` (`local.sorted`) _minvalue)
    (`KismetArrayLibrary.Array_Remove` _output_get _indexofminvalue))
  (return (`local.sorted`)))

(fn `SortMusicLanes`
  (params (musicLanes :type "Array of /Game/Blueprints/Beats/BP_MusicLane Object Reference"))
  (returns (musicLanesOut :type "Array of /Game/Blueprints/Beats/BP_MusicLane Object Reference"))
  (locals (midYValue :type "Float (double-precision)" :default 0.0) (newMusicLanes :type "Array of /Game/Blueprints/Beats/BP_MusicLane Object Reference") (low :type Integer) (high :type Integer) (mid :type Integer))
  (bind _midyvalue (`local.midYValue`))
  (bind _newmusiclanes (`local.newMusicLanes`))
  (for (_array_element _array_index) musicLanes
    (bind (_returnvalue_x _returnvalue_y) (`KismetMathLibrary.BreakVector` (`self.K2_GetActorLocation` _array_element)))
    (if (> _returnvalue_y _midyvalue)
      (set `local.high` _array_index)
      (elif (`KismetMathLibrary.NearlyEqual_FloatFloat` _returnvalue_y _midyvalue)
        (set `local.mid` _array_index)
        (else
          (set `local.low` _array_index)))))
  (`KismetArrayLibrary.Array_Add` _newmusiclanes (`|GetArrayItem` musicLanes (`local.low`)))
  (`KismetArrayLibrary.Array_Add` _newmusiclanes (`|GetArrayItem` musicLanes (`local.mid`)))
  (`KismetArrayLibrary.Array_Add` _newmusiclanes (`|GetArrayItem` musicLanes (`local.high`)))
  (return _newmusiclanes))

(fn `UserConstructionScript`)