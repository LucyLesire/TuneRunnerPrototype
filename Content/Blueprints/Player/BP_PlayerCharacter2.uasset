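; Player character for a lane-based rhythm game where hitting beats adds time and obstacles subtract it.
; Difficulty from the game instance sets the time bonus, Easy auto-hit and tutorial mode.
; Capsule overlaps open a beat window with a delayed grace period for HitBeat, which triggers particle and lane-color feedback.
; Obstacle hits start timed invulnerability, shown by a paused looping timer that flickers the material; Death opens the EndGame level.
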(event `self.ReceiveBeginPlay`
  (`parent.ReceiveBeginPlay`)
  ;[1 1 1] Save sound master
  (bind _returnvalue (`GameplayStatics.GetActorOfClass` "/Game/Blueprints/Sounds/BP_SoundMaster.BP_SoundMaster_C"))
  (set `self.SoundMaster` _returnvalue)
  ;[1 1 1] Initialization of Material change function
  (`KismetSystemLibrary.K2_SetTimer` null "ChangeMaterial" 0.5 true)
  (`KismetSystemLibrary.K2_PauseTimer` null "ChangeMaterial")
  ;[1 1 1] Change variables according to difficulty
  (bind _asbp_game_instance (cast `/Game/Blueprints/Base/BP_GameInstance` (`GameplayStatics.GetGameInstance`)))
  (switch `/Game/Blueprints/Menu/Difficulty` (`/Game/Blueprints/Base/BP_GameInstance.Difficulty` _asbp_game_instance)
    (:`NewEnumerator0`
      (set `self.Easy` true)
      (set `self.AddTime` 3.0))
    (:`NewEnumerator1`
      (set `self.AddTime` 3.0)
      (set `self.Easy` false :!label _label))
    (:`NewEnumerator2`
      (set `self.AddTime` 2.0)
      (goto _label))
    (:`NewEnumerator3`
      (bind _asbp_player_controller (cast `/Game/Blueprints/Player/BP_PLayerController` (`GameplayStatics.GetPlayerController` 0)))
      (set `/Game/Blueprints/Player/BP_PLayerController.Tutorial` true _asbp_player_controller))))

(event `InputAction|FireSecondary`
  (params (Key :type "Key Structure")))

(event `Death`
  ;[1 1 1] Game Over
  (bind _asbp_game_instance (cast `/Game/Blueprints/Base/BP_GameInstance` (`GameplayStatics.GetGameInstance`)))
  (set `/Game/Blueprints/Base/BP_GameInstance.GameOver` true _asbp_game_instance)
  (`self.K2_DestroyActor` self)
  (`GameplayStatics.OpenLevel` "EndGame"))

(event `self.ReceiveTick`
  (params (DeltaSeconds :type "Float (single-precision)"))
  ;[1 1 1] Check if hit => make sure invurnability only lasts max 5s
  (if (`self.HitByObstacle`)
    (bind _output_get (set `self.InvurnableTime` (+ DeltaSeconds (`self.InvurnableTime`))))
    (if (>= _output_get (`self.MaxInvurnableTime`))
      ;[1 1 1] Reset Invurnability
      (set `self.HitByObstacle` false)
      (`KismetSystemLibrary.K2_PauseTimer` null "ChangeMaterial")
      (set `self.InvurnableTime` 0.0)
      (`PrimitiveComponent.SetMaterial` (`self.Mesh`) 0 "/Game/ShooterMannequin/UE4_Mannequin/Materials/M_UE4Man_Body.M_UE4Man_Body")
      (else
        ;[1 1 1] Change material to show invurnability
        (`KismetSystemLibrary.K2_UnPauseTimer` null "ChangeMaterial")))))

(event `self.CapsuleComponent.OnComponentBeginOverlap`
  (params (OverlappedComponent :type "PrimitiveComponent Object Reference") (OtherActor :type "Actor Object Reference") (OtherComp :type "PrimitiveComponent Object Reference") (OtherBodyIndex :type Integer) (bFromSweep :type Boolean) (SweepResult :type "HitResult Structure (by ref)"))
  ;[1 1 1] Beat detection system
  (`/Engine/EditorBlueprintResources/StandardMacros.IsValid` OtherActor
    (:`Is Valid`
      (if (`self.ActorHasTag` OtherActor "Beat")
        (set `self.HittingBeat` true)
        (if (`self.Easy`)
          (bind _asbp_player_controller (cast `/Game/Blueprints/Player/BP_PLayerController` (`GameplayStatics.GetPlayerController` 0)))
          (`self.HitBeat` (`/Game/Blueprints/Player/BP_PLayerController.CurrentLane` _asbp_player_controller)))))))

(event `self.CapsuleComponent.OnComponentEndOverlap`
  (params (OverlappedComponent :type "PrimitiveComponent Object Reference") (OtherActor :type "Actor Object Reference") (OtherComp :type "PrimitiveComponent Object Reference") (OtherBodyIndex :type Integer))
  ;[1 1 1] Beat detection system
  (`/Engine/EditorBlueprintResources/StandardMacros.IsValid` OtherActor
    (:`Is Valid`
      (if (`self.ActorHasTag` OtherActor "Beat")
        ;;[1 1 1] Grace Period
        (`KismetSystemLibrary.Delay` 0.75)
        (set `self.HittingBeat` false)))))

(event `ChangeMaterial`
  (bind _mesh (`self.Mesh`))
  ;[1 1 1] Change material to show invurnability
  (if (== (`|GetArrayItem` (`MeshComponent.GetMaterials` _mesh)) "/Game/ShooterMannequin/UE4_Mannequin/Materials/M_UE4Man_Body.M_UE4Man_Body")
    (`PrimitiveComponent.SetMaterial` _mesh 0 "/Game/ShooterMannequin/UE4_Mannequin/Materials/M_UE4Man_Body_2.M_UE4Man_Body_2")
    (else
      (`PrimitiveComponent.SetMaterial` _mesh 0 "/Game/ShooterMannequin/UE4_Mannequin/Materials/M_UE4Man_Body.M_UE4Man_Body"))))

(event `HitBeat`
  (params (currentLane :type Integer))
  ;[1 1 1] Beat detection system
  (if (`self.HittingBeat`)
    (bind _asbp_game_mode (cast `/Game/Blueprints/Player/BP_GameMode` (`GameplayStatics.GetGameMode`)))
    (`/Game/Blueprints/Player/BP_GameMode.AddTime` _asbp_game_mode (`self.AddTime`))
    (`/Engine/EditorBlueprintResources/StandardMacros.IsValid` (stale `self.CapsuleComponent.OnComponentBeginOverlap` OtherActor)
      (:`Is Valid`
        ;;[1 1 1] Player feedback (Particles)
        (`GameplayStatics.SpawnEmitterAtLocation` "/Game/Blueprints/Particles/P_BeatExplosion.P_BeatExplosion" (`self.K2_GetActorLocation` (stale `self.CapsuleComponent.OnComponentBeginOverlap` OtherActor)))
        (bind _asbp_player_controller (cast `/Game/Blueprints/Player/BP_PLayerController` (`GameplayStatics.GetPlayerController` 0)))
        ;;[1 1 1] Player feedback (Lane Color)
        (`/Game/Blueprints/Beats/BP_MusicLane.ChangeLaneColor` (`|GetArrayItem` (`/Game/Blueprints/Player/BP_PLayerController.MusicLanes` _asbp_player_controller) currentLane) "/Game/Blueprints/Materials/Mat_Lights.Mat_Lights")
        (`/Engine/EditorBlueprintResources/StandardMacros.IncrementInt` (`self.BeatsHit`)
          (:`  `
            (`self.K2_DestroyActor` (stale `self.CapsuleComponent.OnComponentBeginOverlap` OtherActor))
            ;[1 1 1] Change tutorial sequence
            (bind _asbp_game_instance (cast `/Game/Blueprints/Base/BP_GameInstance` (`GameplayStatics.GetGameInstance`)))
            (if (`|EnumEquality` (`/Game/Blueprints/Base/BP_GameInstance.Difficulty` _asbp_game_instance) "NewEnumerator3")
              (bind _currenttutorial (`/Game/Blueprints/Base/BP_GameInstance.CurrentTutorial` _asbp_game_instance))
              (if (== _currenttutorial 1)
                (`/Engine/EditorBlueprintResources/StandardMacros.IncrementInt` _currenttutorial)))))))))

(event `HitObstacle`
  ;[1 1 1] Obstacle detection system
  (bind _asbp_player_controller (cast `/Game/Blueprints/Player/BP_PLayerController` (`GameplayStatics.GetPlayerController` 0)))
  ;;[1 1 1] Check if in powerup or recently hit by obstacle
  (if (not (or (`/Game/Blueprints/Player/BP_PLayerController.3LanesPowerup` _asbp_player_controller) (`self.HitByObstacle`)))
    ;;[1 1 1] Decrease timer
    (bind _asbp_game_mode (cast `/Game/Blueprints/Player/BP_GameMode` (`GameplayStatics.GetGameMode`)))
    (`/Game/Blueprints/Player/BP_GameMode.AddTime` _asbp_game_mode (* -1 (`self.MaxInvurnableTime`)))
    (set `self.HitByObstacle` true)))

(fn `Slowdowntimepowerup`
  (params (SlowDownTime :type Boolean))
  (if SlowDownTime
    (`/Game/Blueprints/Sounds/BP_SoundMaster.SlowDownTime` (`self.SoundMaster`))))

(fn `UserConstructionScript`
  (`parent.UserConstructionScript`))