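; Player controller for a three-lane music game that handles lane switching, beat hits, tutorial progress on movement and Escape to the main menu.
; It starts the pawn in a random lane from the game mode's MusicLanes and moves it between lane sockets.
; The 3Lanes power-up locks movement and spawns re-skinned characters in the other lanes, so HitBeat checks every lane.
; A Delay on Tick later destroys those extra characters.
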(event `InputAction|Escape`
  (params (Key :type "Key Structure"))
  (:`Pressed`
    (`GameplayStatics.OpenLevel` "MainMenu")))

(event `InputAction|MoveLaneRight`
  (params (Key :type "Key Structure"))
  ;[1 1 1] Handle Movement Input
  (:`Pressed`
    (`self.MoveLane` false)
    ;[1 1 1] Tutorial
    (if (`self.Tutorial`) :!label _label
      (bind _asbp_game_instance (cast `/Game/Blueprints/Base/BP_GameInstance` (`GameplayStatics.GetGameInstance`)))
      (if (== (`/Game/Blueprints/Base/BP_GameInstance.CurrentTutorial` _asbp_game_instance) 0)
        (set `/Game/Blueprints/Base/BP_GameInstance.CurrentTutorial` 1 _asbp_game_instance)))))

(event `InputAction|MoveLaneLeft`
  (params (Key :type "Key Structure"))
  ;[1 1 1] Handle Movement Input
  (:`Pressed`
    (`self.MoveLane` true)
    (goto _label)))

(event `SetRandomLane`
  ;[1 1 1] Get Random Lane
  (bind _asbp_game_mode (cast `/Game/Blueprints/Player/BP_GameMode` (`GameplayStatics.GetGameMode`)))
  (bind _output_get (set `self.MusicLanes` (`/Game/Blueprints/Player/BP_GameMode.MusicLanes` _asbp_game_mode)))
  (set `self.CurrentLane` (`.OutIndex` (`KismetArrayLibrary.Array_Random` _output_get)))
  (for (_array_element _array_index) (`self.MusicLanes`)
    (if (== _array_index (`self.CurrentLane`))
      (bind _playersocket (`/Game/Blueprints/Beats/BP_MusicLane.PlayerSocket` _array_element))
      ;[1 1 1] Move player to correct start lane
      (`self.K2_SetActorTransform` (`self.K2_GetPawn`) (`KismetMathLibrary.MakeTransform` (`SceneComponent.GetSocketLocation` _playersocket "None") (`SceneComponent.GetSocketRotation` _playersocket "None")) false true))))

(event `3Lanes`
  (bind _extraplayers (`self.ExtraPlayers`))
  (bind _extraplayers_2 (`self.ExtraPlayers`))
  (bind _extraplayers_3 (`self.ExtraPlayers`))
  (bind _currentlane (`self.CurrentLane`))
  (bind _musiclanes (`self.MusicLanes`))
  (bind _returnvalue (`SceneComponent.K2_GetComponentLocation` (`/Game/Blueprints/Beats/BP_MusicLane.PlayerSocket` (`|GetArrayItem` _musiclanes 1))))
  (bind _returnvalue_2 (`SceneComponent.K2_GetComponentLocation` (`/Game/Blueprints/Beats/BP_MusicLane.PlayerSocket` (`|GetArrayItem` _musiclanes 2))))
  (bind _returnvalue_3 (`SceneComponent.K2_GetComponentLocation` (`/Game/Blueprints/Beats/BP_MusicLane.PlayerSocket` (`|GetArrayItem` _musiclanes))))
  ;[1 1 1] 3 lanes power-up
  (if (not (`self.3LanesPowerup`))
    (`KismetSystemLibrary.Delay` 0.2)
    (if (== _currentlane 0)
      (bind _returnvalue_4 (`|SpawnActorFromClass` "/Game/Blueprints/Player/BP_PlayerCharacter2.BP_PlayerCharacter2_C" (`KismetMathLibrary.MakeTransform` _returnvalue) "Undefined" "OverrideRootScale" null null))
      (bind _returnvalue_5 (`|SpawnActorFromClass` "/Game/Blueprints/Player/BP_PlayerCharacter2.BP_PlayerCharacter2_C" (`KismetMathLibrary.MakeTransform` _returnvalue_2) "Undefined" "OverrideRootScale" null null))
      (bind _asbp_player_character_2 (cast `/Game/Blueprints/Player/BP_PlayerCharacter2` (`GameplayStatics.GetPlayerCharacter` 0)))
      (`KismetArrayLibrary.Array_Add` _extraplayers _asbp_player_character_2)
      (`KismetArrayLibrary.Array_Add` _extraplayers _returnvalue_4)
      (`KismetArrayLibrary.Array_Add` _extraplayers _returnvalue_5)
      (elif (== _currentlane 1)
        (bind _returnvalue_6 (`|SpawnActorFromClass` "/Game/Blueprints/Player/BP_PlayerCharacter2.BP_PlayerCharacter2_C" (`KismetMathLibrary.MakeTransform` _returnvalue_3) "Undefined" "OverrideRootScale" null null))
        (bind _returnvalue_7 (`|SpawnActorFromClass` "/Game/Blueprints/Player/BP_PlayerCharacter2.BP_PlayerCharacter2_C" (`KismetMathLibrary.MakeTransform` _returnvalue_2) "Undefined" "OverrideRootScale" null null))
        (`KismetArrayLibrary.Array_Add` _extraplayers_3 _returnvalue_6)
        (bind _asbp_player_character_2_2 (cast `/Game/Blueprints/Player/BP_PlayerCharacter2` (`GameplayStatics.GetPlayerCharacter` 0)))
        (`KismetArrayLibrary.Array_Add` _extraplayers_3 _asbp_player_character_2_2)
        (`KismetArrayLibrary.Array_Add` _extraplayers_3 _returnvalue_7)
        (else
          (bind _returnvalue_8 (`|SpawnActorFromClass` "/Game/Blueprints/Player/BP_PlayerCharacter2.BP_PlayerCharacter2_C" (`KismetMathLibrary.MakeTransform` _returnvalue_3) "Undefined" "OverrideRootScale" null null))
          (bind _returnvalue_9 (`|SpawnActorFromClass` "/Game/Blueprints/Player/BP_PlayerCharacter2.BP_PlayerCharacter2_C" (`KismetMathLibrary.MakeTransform` _returnvalue) "Undefined" "OverrideRootScale" null null))
          (`KismetArrayLibrary.Array_Add` _extraplayers_2 _returnvalue_8)
          (`KismetArrayLibrary.Array_Add` _extraplayers_2 _returnvalue_9)
          (bind _asbp_player_character_2_3 (cast `/Game/Blueprints/Player/BP_PlayerCharacter2` (`GameplayStatics.GetPlayerCharacter` 0)))
          (`KismetArrayLibrary.Array_Add` _extraplayers_2 _asbp_player_character_2_3))))
    (set `self.3LanesPowerup` true)
    (for (_array_element _array_index) (`self.ExtraPlayers`)
      (if (not (== _array_index (`self.CurrentLane`)))
        (`PrimitiveComponent.SetMaterial` (`Character.Mesh` _array_element) 0 "/Game/ShooterMannequin/UE4_Mannequin/Materials/M_UE4Man_Body_3.M_UE4Man_Body_3")))))

(event `self.ReceiveTick`
  (params (DeltaSeconds :type "Float (single-precision)"))
  (bind _extraplayers (`self.ExtraPlayers`))
  ;[1 1 1] Reset 3 Lanes powerup
  (if (`self.3LanesPowerup`)
    (`KismetSystemLibrary.Delay` 5.0)
    (set `self.3LanesPowerup` false)
    (for (_array_element _array_index) _extraplayers
      (if (not (== _array_index (`self.CurrentLane`)))
        (`self.K2_DestroyActor` _array_element)))
    (`KismetArrayLibrary.Array_Clear` _extraplayers)))

(event `self.ReceiveBeginPlay`
  ;[1 1 1] Reset 3 Lanes powerup
  (`self.SetRandomLane`))

(event `InputAction|HitBeat`
  (params (Key :type "Key Structure"))
  ;[1 1 1] Check if hitting a beat
  (:`Pressed`
    (if (`self.3LanesPowerup`)
      ;;[1 1 1] Check during 3 Lanes powerup
      (for (_array_element _array_index) (`self.ExtraPlayers`)
        (`/Game/Blueprints/Player/BP_PlayerCharacter2.HitBeat` _array_element _array_index))
      (else
        (bind _asbp_player_character_2 (cast `/Game/Blueprints/Player/BP_PlayerCharacter2` (`GameplayStatics.GetPlayerPawn` 0)))
        (`/Game/Blueprints/Player/BP_PlayerCharacter2.HitBeat` _asbp_player_character_2 (`self.CurrentLane`))))))

(fn `MoveLane`
  (params (Right :type Boolean))
  (locals (MoveToLane :type Integer))
  (if (not (`self.3LanesPowerup`))
    ;[1 1 1] Set move to lane
    (if Right
      (set `local.MoveToLane` (`KismetMathLibrary.Clamp` (+ (`self.CurrentLane`) 1) 0 2))
      (else
        (set `local.MoveToLane` (`KismetMathLibrary.Clamp` (- (`self.CurrentLane`) 1) 0 2))))
    (if (!= (`local.MoveToLane`) (`self.CurrentLane`))
      ;[1 1 1] Get player socket and move player to that lane
      (for (_array_element _array_index) (`self.MusicLanes`)
        (if (== _array_index (`local.MoveToLane`))
          (bind _playersocket (`/Game/Blueprints/Beats/BP_MusicLane.PlayerSocket` _array_element))
          (`self.K2_SetActorTransform` (`self.K2_GetPawn`) (`KismetMathLibrary.MakeTransform` (`SceneComponent.GetSocketLocation` _playersocket "None") (`SceneComponent.GetSocketRotation` _playersocket "None")) false false)
          (set `self.CurrentLane` (`local.MoveToLane`)))))))

(fn `UserConstructionScript`)