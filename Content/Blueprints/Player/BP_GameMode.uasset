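; BP_GameMode is the game mode for a lane-based music game in which a countdown timer serves as the player's survival resource.
; Tick drains TimeLeft and calls Death on the player character once it runs out, while AddTime adjusts it on beat hits or obstacles.
; RespawnPlayer spawns the default pawn at a player start, possesses it and has the player controller pick a random lane.
; BeginPlay caches all BP_MusicLane actors.
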(event `self.ReceiveBeginPlay`
  (bind _outactors (`GameplayStatics.GetAllActorsOfClass` "/Game/Blueprints/Beats/BP_MusicLane.BP_MusicLane_C"))
  (set `self.MusicLanes` _outactors))

(event `self.ReceiveTick`
  (params (DeltaSeconds :type "Float (single-precision)"))
  ;[1 1 1] Decrease timer
  (bind _output_get (set `self.TimeLeft` (- (`self.TimeLeft`) DeltaSeconds)))
  ;[1 1 1] Check for dead => restart
  (if (<= _output_get 0.0)
    (bind _asbp_player_character_2 (cast `/Game/Blueprints/Player/BP_PlayerCharacter2` (`GameplayStatics.GetPlayerCharacter` 0)))
    (`/Game/Blueprints/Player/BP_PlayerCharacter2.Death` _asbp_player_character_2)))

(event `RespawnPlayer`
  (bind _returnvalue (`GameplayStatics.GetPlayerController` 0))
  ;[1 1 1] Respawn player
  (bind _returnvalue_2 (`|SpawnActorFromClass` (`self.DefaultPawnClass`) (`self.GetTransform` (`self.K2_FindPlayerStart` _returnvalue)) "Undefined" "OverrideRootScale" null null))
  (`Controller.Possess` _returnvalue _returnvalue_2)
  (bind _asbp_player_controller (cast `/Game/Blueprints/Player/BP_PLayerController` _returnvalue))
  (`/Game/Blueprints/Player/BP_PLayerController.SetRandomLane` _asbp_player_controller))

(event `AddTime`
  (params (Time :type "Float (double-precision)" :default 0.0))
  ;[1 1 1] Change timer on beat hit or obstacle
  (set `self.TimeLeft` (+ Time (`self.TimeLeft`))))

(fn `UserConstructionScript`)