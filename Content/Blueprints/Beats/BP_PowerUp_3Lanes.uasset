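; BP_PowerUp_3Lanes is a pickup actor that grants the player the three-lane power-up.
; When its Box component is overlapped by an actor carrying the player tag, it casts player controller 0 to BP_PlayerController and calls its 3Lanes function.
; The pickup then destroys itself, leaving the effect itself to the controller.
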(event `self.Box.OnComponentBeginOverlap`
  (params (OverlappedComponent :type "PrimitiveComponent Object Reference") (OtherActor :type "Actor Object Reference") (OtherComp :type "PrimitiveComponent Object Reference") (OtherBodyIndex :type Integer) (bFromSweep :type Boolean) (SweepResult :type "HitResult Structure (by ref)"))
  ;[1 1 1] Give player powerup
  (`/Engine/EditorBlueprintResources/StandardMacros.IsValid` OtherActor
    (:`Is Valid`
      (if (`self.ActorHasTag` OtherActor (`self.PlayerTag`))
        (bind _asbp_player_controller (cast `/Game/Blueprints/Player/BP_PLayerController` (`GameplayStatics.GetPlayerController` 0)))
        (`/Game/Blueprints/Player/BP_PLayerController.3Lanes` _asbp_player_controller)
        (`self.K2_DestroyActor`)))))

(fn `UserConstructionScript`
  (`parent.UserConstructionScript`))