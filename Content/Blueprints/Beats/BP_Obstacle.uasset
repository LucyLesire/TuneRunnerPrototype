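; BP_Obstacle is a hazard actor that spins and penalizes the player on contact.
; Every tick it rolls its Box component at a constant, frame-rate-independent speed.
; When the Box begins overlapping a valid actor with the player tag, it casts to BP_PlayerCharacter2 and calls HitObstacle, leaving the damage response to the character.
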(event `self.ReceiveTick`
  (params (DeltaSeconds :type "Float (single-precision)"))
  ;[1 1 1] RotationAnimation
  (`parent.ReceiveTick` DeltaSeconds)
  (`SceneComponent.K2_AddLocalRotation` (`self.Box`) (`KismetMathLibrary.MakeRotator` (* DeltaSeconds 1000.0)) false false))

(event `self.Box.OnComponentBeginOverlap`
  (params (OverlappedComponent :type "PrimitiveComponent Object Reference") (OtherActor :type "Actor Object Reference") (OtherComp :type "PrimitiveComponent Object Reference") (OtherBodyIndex :type Integer) (bFromSweep :type Boolean) (SweepResult :type "HitResult Structure (by ref)"))
  ;[1 1 1] Deal damage to player
  (`/Engine/EditorBlueprintResources/StandardMacros.IsValid` OtherActor
    (:`Is Valid`
      (if (`self.ActorHasTag` OtherActor (`self.PlayerTag`))
        (bind _asbp_player_character_2 (cast `/Game/Blueprints/Player/BP_PlayerCharacter2` OtherActor))
        (`/Game/Blueprints/Player/BP_PlayerCharacter2.HitObstacle` _asbp_player_character_2)))))

(fn `UserConstructionScript`
  (`parent.UserConstructionScript`))