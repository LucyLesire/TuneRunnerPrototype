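; BP_MusicLane is a lane in a music game that spawns beats, obstacles and power-ups at its BeatSocket.
; Spawn events create each item type, with power-ups choosing randomly between two spawn branches.
; Items leaving BeatDestroyCollision are destroyed by tag, and a missed beat also deducts game mode time and increments the game instance's missed count.
; ChangeLaneColor briefly swaps both lane meshes' material for feedback, then resets it.
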(event `self.ReceiveTick`
  (params (DeltaSeconds :type "Float (single-precision)")))

(event `self.BeatDestroyCollision.OnComponentEndOverlap`
  (params (OverlappedComponent :type "PrimitiveComponent Object Reference") (OtherActor :type "Actor Object Reference") (OtherComp :type "PrimitiveComponent Object Reference") (OtherBodyIndex :type Integer))
  ;[1 1 1] Destroy beat and remove time
  (`/Engine/EditorBlueprintResources/StandardMacros.IsValid` OtherActor
    (:`Is Valid`
      (if (`self.ActorHasTag` OtherActor (`self.BeatTag`))
        (`self.K2_DestroyActor` OtherActor)
        (bind _asbp_game_mode (cast `/Game/Blueprints/Player/BP_GameMode` (`GameplayStatics.GetGameMode`)))
        (`/Game/Blueprints/Player/BP_GameMode.AddTime` _asbp_game_mode -5.0)
        (`self.ChangeLaneColor` "/Game/Blueprints/Materials/Mat_Lights_3.Mat_Lights_3")
        ;[1 1 1] Keep track of stats
        (bind _asbp_game_instance (cast `/Game/Blueprints/Base/BP_GameInstance` (`GameplayStatics.GetGameInstance`)))
        (`/Engine/EditorBlueprintResources/StandardMacros.IncrementInt` (`/Game/Blueprints/Base/BP_GameInstance.BeatsMissed` _asbp_game_instance))
        (elif (`self.ActorHasTag` OtherActor (`self.ObstacleTag`))
          (`self.K2_DestroyActor` OtherActor)
          (elif (`self.ActorHasTag` OtherActor (`self.PowerUpTag`))
            (`self.K2_DestroyActor` OtherActor)))))))

(event `ChangeLaneColor`
  (params (Material :type "MaterialInterface Object Reference"))
  ;[1 1 1] Player feedback on hit
  (`PrimitiveComponent.SetMaterial` (`self.StaticMesh`) 0 Material)
  (`PrimitiveComponent.SetMaterial` (`self.StaticMesh1`) 0 Material)
  ;;[1 1 1] Reset
  (`KismetSystemLibrary.Delay` 0.5)
  (`PrimitiveComponent.SetMaterial` (`self.StaticMesh`) 0 "/Game/Blueprints/Materials/Mat_Lights_2.Mat_Lights_2")
  (`PrimitiveComponent.SetMaterial` (`self.StaticMesh1`) 0 "/Game/Blueprints/Materials/Mat_Lights_2.Mat_Lights_2"))

(event `SpawnBeats`
  ;[1 1 1] Spawn Items
  (`|SpawnActorFromClass` "/Game/Blueprints/Beats/BP_Beat.BP_Beat_C" (`KismetMathLibrary.MakeTransform` (`SceneComponent.K2_GetComponentLocation` (`self.BeatSocket`))) "Undefined" "OverrideRootScale" null null))

(event `SpawnObstacle`
  ;[1 1 1] Spawn Items
  (`|SpawnActorFromClass` "/Game/Blueprints/Beats/BP_Obstacle.BP_Obstacle_C" (`KismetMathLibrary.MakeTransform` (`SceneComponent.K2_GetComponentLocation` (`self.BeatSocket`))) "Undefined" "OverrideRootScale" null null))

(event `SpawnPowerUp`
  (bind _returnvalue (`SceneComponent.K2_GetComponentLocation` (`self.BeatSocket`)))
  ;[1 1 1] Spawn Items
  (if (`KismetMathLibrary.RandomBool`)
    (`|SpawnActorFromClass` "/Game/Blueprints/Beats/BP_PowerUp_3Lanes.BP_PowerUp_3Lanes_C" (`KismetMathLibrary.MakeTransform` _returnvalue) "Undefined" "OverrideRootScale" null null)
    (else
      (`|SpawnActorFromClass` "/Script/Mechanics_LucyLesire.SlowDownPowerUp" (`KismetMathLibrary.MakeTransform` _returnvalue (struct) (1.0 1.0 1.0)) "Undefined" "OverrideRootScale" null null))))

(fn `UserConstructionScript`)